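; BP_Pistol is a pickup weapon Blueprint that attaches to the character who picks it up.
; The TP_PickUp OnPickUp event passes that character to the TPWeapon component's AttachWeapon.
; The construction script gives TPWeapon an SMG11 skeletal mesh despite the pistol name and a reference back to this Blueprint.
; It also derives the time between shots as the reciprocal of the fire rate.
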(event `self.TP_PickUp.OnPickUp`
  (params (PickUpCharacter :type "GR2_ReworkCharacter Object Reference"))
  (`TP_WeaponComponent.AttachWeapon` (`self.TP_Weapon`) PickUpCharacter))

(fn `UserConstructionScript`
  (bind _tp_weapon (`self.TP_Weapon`))
  (`SkeletalMeshComponent.SetSkeletalMeshAsset` _tp_weapon "/Game/FPS_Weapon_Bundle/Weapons/Meshes/SMG11/SK_SMG11_Y.SK_SMG11_Y")
  (set `TP_WeaponComponent.WeaponBlueprint` self _tp_weapon)
  (set `self.TimeBetweenShots` (/ 1.0 (`KismetMathLibrary.Conv_IntToDouble` (`self.FireRate`)))))