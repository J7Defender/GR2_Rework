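; AK47 weapon Blueprint that attaches to the character who picks it up, through its BPWeaponComponent.
; The construction script sets the component's skeletal mesh, links component and weapon to each other, and derives the time between shots from the fire rate.
; UpdateAmmoUI pushes current and remaining ammo to the owner's in-match HUD widget.
; UpdateReloadUI is a stub that only casts the HUD.
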(event `self.TP_PickUp.OnPickUp`
  (params (PickUpCharacter :type "GR2_ReworkCharacter Object Reference"))
  (`TP_WeaponComponent.AttachWeapon` (`self.BP_WeaponComponent`) PickUpCharacter))

(event `self.UpdateAmmoUI`
  (bind _asbp_widget_in_match (cast `/Game/HUD/Menu/BP_Widget_InMatch` (`GR2_ReworkCharacter.CharacterHUD` (`TP_WeaponComponent.Character` (`self.BP_WeaponComponent`)))))
  (`/Game/HUD/Menu/BP_Widget_InMatch.UpdateAmmoUI` _asbp_widget_in_match (`KismetStringLibrary.Conv_IntToString` (`self.CurrentAmmo`)) (`KismetStringLibrary.Conv_IntToString` (`self.RemainingAmmo`))))

(event `self.UpdateReloadUI`
  (cast `/Game/HUD/Menu/BP_Widget_InMatch` (`GR2_ReworkCharacter.CharacterHUD` (`TP_WeaponComponent.Character` (`self.BP_WeaponComponent`)))))

(fn `UserConstructionScript`
  (bind _bp_weaponcomponent (`self.BP_WeaponComponent`))
  (`SkeletalMeshComponent.SetSkeletalMeshAsset` _bp_weaponcomponent "/Game/FPS_Weapon_Bundle/Weapons/Meshes/Ka47/SK_KA47.SK_KA47")
  (set `TP_WeaponComponent.WeaponBlueprint` self _bp_weaponcomponent)
  (set `self.WeaponComponent` (`self.BP_WeaponComponent`))
  (set `self.TimeBetweenShots` (/ 1.0 (`KismetMathLibrary.Conv_IntToDouble` (`self.FireRate`)))))