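; Weapon Blueprint that pairs with a weapon component and reports its ammo and reload state to the in-match HUD.
; The construction script links itself and BPWeaponComponent to each other and derives the time between shots from the fire rate.
; Two UI events cast the owning character's HUD to BP_Widget_InMatch to update ammo text and toggle the reloading indicator.
; Firing and reload logic are absent from these graphs.
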(event `self.UpdateAmmoUI`
  (bind _asbp_widget_in_match (cast `/Game/HUD/BP_Widget_InMatch` (`GR2_ReworkCharacter.CharacterHUD` (`TP_WeaponComponent.Character` (`self.BP_WeaponComponent`)))))
  (`/Game/HUD/BP_Widget_InMatch.UpdateAmmoUI` _asbp_widget_in_match (`KismetStringLibrary.Conv_IntToString` (`self.CurrentAmmo`)) (`KismetStringLibrary.Conv_IntToString` (`self.RemainingAmmo`))))

(event `self.UpdateReloadUI`
  (bind _asbp_widget_in_match (cast `/Game/HUD/BP_Widget_InMatch` (`GR2_ReworkCharacter.CharacterHUD` (`TP_WeaponComponent.Character` (`self.BP_WeaponComponent`)))))
  (if (`self.bIsReloading`)
    (set `/Game/HUD/BP_Widget_InMatch.ReloadingVisible` "Visible" _asbp_widget_in_match)
    (else
      (set `/Game/HUD/BP_Widget_InMatch.ReloadingVisible` "Hidden" _asbp_widget_in_match))))

(fn `UserConstructionScript`
  (set `TP_WeaponComponent.WeaponBlueprint` self (`self.BP_WeaponComponent`))
  (set `self.WeaponComponent` (`self.BP_WeaponComponent`))
  (set `self.TimeBetweenShots` (/ 1.0 (`KismetMathLibrary.Conv_IntToDouble` (`self.FireRate`)))))