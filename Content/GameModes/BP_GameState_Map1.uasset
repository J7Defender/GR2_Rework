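; Game state for Map1 that runs the match countdown and relays match info to the in-match HUD.
; Tick uses a one-second Delay to decrement RemainingTime; once it drops below zero, the server calls TryChangeMatchState on GR2_ReworkGameState_Map1.
; Score, timer, winner and match-state events run only off-server, updating BP_Widget_InMatch through player 0's character HUD.
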(event `self.ReceiveTick`
  (params (DeltaSeconds :type "Float (single-precision)"))
  ;[1 1 1] Count Down Timer
  (`KismetSystemLibrary.Delay` 1.0)
  (`KismetSystemLibrary.PrintString` (`KismetStringLibrary.Concat_StrStr` "Remaining Time: " (`KismetStringLibrary.Conv_IntToString` (`self.RemainingTime`))) false)
  (if (>= (`self.RemainingTime`) 0)
    (bind _output_get (set `self.RemainingTime` (- (`self.RemainingTime`) 1)))
    (`self.UpdateTimerUI` _output_get)
    (else
      ;;[1 1 1] Try to Change Match State
      (bind _asgr2_rework_game_state_map_1 (cast `GR2_ReworkGameState_Map1` (`GameplayStatics.GetGameState`)))
      (if (`KismetSystemLibrary.IsServer`)
        (`self.TryChangeMatchState` _asgr2_rework_game_state_map_1)))))

(event `self.UpdateScoreUI`
  (params (FRedTeamScore :type Integer) (FBlueTeamScore :type Integer))
  ;[1 1 1] Update Score on User Interface
  (if (not (`KismetSystemLibrary.IsServer`))
    (bind _asgr2_rework_character (`self.Get Current Client Character`))
    (bind _characterhud (`GR2_ReworkCharacter.CharacterHUD` _asgr2_rework_character))
    (if (`KismetSystemLibrary.IsValid` _characterhud)
      (bind _asbp_widget_in_match (cast `/Game/HUD/Menu/BP_Widget_InMatch` _characterhud))
      (`/Game/HUD/Menu/BP_Widget_InMatch.UpdateScoreUI` _asbp_widget_in_match (`KismetStringLibrary.Conv_IntToString` FRedTeamScore) (`KismetStringLibrary.Conv_IntToString` FBlueTeamScore)))))

(event `self.UpdateTimerUI`
  (params (FRemainingTime :type Integer))
  ;[1 1 1] Update Timer on UI
  (if (not (`KismetSystemLibrary.IsServer`))
    (bind _asgr2_rework_character (`self.Get Current Client Character`))
    (bind _characterhud (`GR2_ReworkCharacter.CharacterHUD` _asgr2_rework_character))
    (if (`KismetSystemLibrary.IsValid` _characterhud)
      (bind _asbp_widget_in_match (cast `/Game/HUD/Menu/BP_Widget_InMatch` _characterhud))
      (`/Game/HUD/Menu/BP_Widget_InMatch.UpdateTimerUI` _asbp_widget_in_match (`KismetStringLibrary.Conv_IntToString` (`KismetMathLibrary.Max` FRemainingTime))))))

(event `self.UpdateWinnerUI`
  (params (WinnerIndex :type Integer))
  ;[1 1 1] Show Winner UI at post match
  (if (not (`KismetSystemLibrary.IsServer`))
    (bind _asgr2_rework_character (`self.Get Current Client Character`))
    (bind _characterhud (`GR2_ReworkCharacter.CharacterHUD` _asgr2_rework_character))
    (if (`KismetSystemLibrary.IsValid` _characterhud)
      (bind _asbp_widget_in_match (cast `/Game/HUD/Menu/BP_Widget_InMatch` _characterhud))
      (`/Game/HUD/Menu/BP_Widget_InMatch.UpdateWinningUI` _asbp_widget_in_match WinnerIndex))))

(event `self.UpdateMatchStateUI`
  (params (FMatchState :type "EMatchState Enum" :default "E_Default"))
  ;[1 1 1] Change Curent MatchState on UI on MatchState update
  (if (not (`KismetSystemLibrary.IsServer`))
    (bind _asgr2_rework_character (`self.Get Current Client Character`))
    (bind _characterhud (`GR2_ReworkCharacter.CharacterHUD` _asgr2_rework_character))
    (if (`KismetSystemLibrary.IsValid` _characterhud)
      (bind _asbp_widget_in_match (cast `/Game/HUD/Menu/BP_Widget_InMatch` _characterhud))
      (`/Game/HUD/Menu/BP_Widget_InMatch.UpdateMatchStateUI` _asbp_widget_in_match FMatchState))))

(fn `Get Current Client Character`
  (returns (`AsGR2 Rework Character` :type "GR2_ReworkCharacter Object Reference"))
  (bind _asgr2_rework_character (cast `GR2_ReworkCharacter` (`GameplayStatics.GetPlayerCharacter` 0)))
  (return _asgr2_rework_character))

(fn `UserConstructionScript`)